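; Corridor tile for a runner course that asks Run_GameMode to add the next tile when RunPlayer hits EndTrigger, then destroys itself after a delay.
; Construction skips obstacles on the first few tiles, then randomly adds a child actor at one of three spawn points.
; Game mode counters cap the course length and drive the end-of-run widget, while a HasSpawned flag guards against double spawns.
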(event OnComponentBeginOverlap(EndTrigger)
  (params (OverlappedComponent :type Primitive%20Component%20Object%20Reference) (OtherActor :type Actor%20Object%20Reference) (OtherComp :type Primitive%20Component%20Object%20Reference) (OtherBodyIndex :type Integer) (bFromSweep :type Boolean) (SweepResult :type Hit%20Result%20Structure%20%28by%20ref%29))
  ;[1 1 1] Casts
  (bind _asrun_game_mode (|Casts OtherActor))
  ;[1 1 1] Prevents The Course From Spawning Infinitely (Infinite Loop Prevention)
  (bind _infinitykiller (|InfinityKiller _asrun_game_mode)
    (:then
      ;[1 1 1] Recognizes Corridors No Longer Spawning And Spawns Widget To Signify End Of The Course
      (|CourseEnd _asrun_game_mode _asrun_game_mode))
    (:else
      ;[1 1 1] Without This, Each New Tile Spawn Will Spawn Two New Corridors. This Is The Fix To Spawn Only One New Corridor At A Time.
      (|SingleCorridorSpawn _asrun_game_mode
        (:then
          ;[1 1 1] Resets Spawn Condition
          (Variables|/Game/Run_GameMode.Run_GameMode_C|SetHasSpawned _asrun_game_mode false))
        (:else
          ;[1 1 1] Increments Infinite Loop Failsafe
          (|FailsafeIncrement _asrun_game_mode _infinitykiller)
          ;[1 1 1] Increments Variation Index
          (|VariationIndexIncrement _asrun_game_mode _asrun_game_mode)
          ;[1 1 1] Adds New Corridor
          (Default|AddFloorTile _asrun_game_mode)
          ;[1 1 1] Destroys Current Corridor After Delay
          (Utilities|FlowControl|Delay 5.0)
          (Actor|DestroyActor))))))

(fn ConstructionScript
  (CallFunction|SetSpawnPoints)
  (CallFunction|SpawnBlocker))

(fn GetAttachTransform
  (return (Transformation|GetWorldTransform (Variables|Default|GetAttach%20Point))))

(fn SetSpawnPoints
  (Variables|Default|SetSpawnPoints (Utilities|Array|MakeArray (Transformation|GetRelativeTransform (Variables|Default|GetSpawnPoint)) (Transformation|GetRelativeTransform (Variables|Default|GetSpawnPointL)) (Transformation|GetRelativeTransform (Variables|Default|GetSpawnPointR)))))

(fn SpawnBlocker
  (bind _spawnpoints (Variables|Default|GetSpawnPoints))
  (bind _returnvalue (Utilities|Array|LastIndex _spawnpoints))
  (bind _returnvalue_2 (Math|Random|RandomIntegerinRange 0 _returnvalue))
  (bind _output (Utilities|Array|Get(acopy) _spawnpoints _returnvalue_2))
  (bind _asrun_game_mode (Utilities|Casting|CastToRun_GameMode (Game|GetGameMode)))
  (if (<= (Variables|/Game/Run_GameMode.Run_GameMode_C|GetSpawnDelay _asrun_game_mode) 6)
    (Variables|/Game/Run_GameMode.Run_GameMode_C|SetSpawnDelay _asrun_game_mode (+ (Variables|/Game/Run_GameMode.Run_GameMode_C|GetSpawnDelay _asrun_game_mode) 1))
    (else
      (switch int (Math|Random|RandomIntegerinRange 0 2)
        (:1
          _)
        (:2
          _))
      (switch int (Math|Random|RandomIntegerinRange 0 12)
        (:Default
          (AddComponent|AddChildActorComponent false _output :!label _label))
        (:0
          (AddComponent|AddChildActorComponent false _output))
        (:1
          (AddComponent|AddChildActorComponent false _output))
        (:2
          (AddComponent|AddChildActorComponent false _output))
        (:3
          (AddComponent|AddChildActorComponent false _output))
        (:4
          (AddComponent|AddChildActorComponent false _output))
        (:5
          (AddComponent|AddChildActorComponent false _output))
        (:6
          (AddComponent|AddChildActorComponent false _output))
        (:7
          (AddComponent|AddChildActorComponent false _output))
        (:8
          (AddComponent|AddChildActorComponent false _output))
        (:9
          (AddComponent|AddChildActorComponent false _output))
        (:10
          (AddComponent|AddChildActorComponent false _output))
        (:11
          (AddComponent|AddChildActorComponent false _output))
        (:12
          (goto _label))))))