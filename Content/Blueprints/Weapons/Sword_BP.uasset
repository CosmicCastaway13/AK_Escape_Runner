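; Sword weapon Blueprint that damages BasicEnemy actors during a swing.
; Swing enables its Collision component for query-only overlaps, then disables it after a one-second delay.
; On overlap it ignores the Player, asks the player character's CalcDamage for the amount, applies it to the enemy, and turns collision off so a hit registers only once.
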(event OnComponentBeginOverlap(Collision)
  (params (OverlappedComponent :type Primitive%20Component%20Object%20Reference) (OtherActor :type Actor%20Object%20Reference) (OtherComp :type Primitive%20Component%20Object%20Reference) (OtherBodyIndex :type Integer) (bFromSweep :type Boolean) (SweepResult :type Hit%20Result%20Structure%20%28by%20ref%29))
  (Utilities|Casting|CastToPlayer OtherActor
    (:CastFailed
      (bind _asbasic_enemy (Utilities|Casting|CastToBasicEnemy OtherActor))
      (bind _asplayer (Utilities|Casting|CastToPlayer (Game|GetPlayerCharacter 0)))
      (bind _damage (Default|CalcDamage _asplayer))
      (Default|TakeDamage _asbasic_enemy _damage)
      (Collision|SetCollisionEnabled (Variables|Default|GetCollision) "NoCollision"))))

(event Custom|Swing
  (Collision|SetCollisionEnabled (Variables|Default|GetCollision) "QueryOnly")
  (Utilities|FlowControl|Delay 1.0)
  (Collision|SetCollisionEnabled (Variables|Default|GetCollision) "NoCollision"))

(fn ConstructionScript
  (|CallParentFunction))