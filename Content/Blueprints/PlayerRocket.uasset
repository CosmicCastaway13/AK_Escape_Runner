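; PlayerRocket is a player projectile that explodes on contact and damages a BasicEnemy.
; Hitbox overlaps with anything other than the Player or another rocket trigger Explode, which spawns a flame effect and briefly enables the query-only Explosion collider, off since construction.
; The first BasicEnemy overlapping that collider takes damage and the rocket is destroyed immediately; otherwise it self-destroys after a short delay.
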(event OnComponentBeginOverlap(Hitbox)
  (params (OverlappedComponent :type Primitive%20Component%20Object%20Reference) (OtherActor :type Actor%20Object%20Reference) (OtherComp :type Primitive%20Component%20Object%20Reference) (OtherBodyIndex :type Integer) (bFromSweep :type Boolean) (SweepResult :type Hit%20Result%20Structure%20%28by%20ref%29))
  (Utilities|Casting|CastToPlayer OtherActor
    (:CastFailed
      (Utilities|Casting|CastToPlayerRocket OtherActor
        (:CastFailed
          (CallFunction|Explode))))))

(event OnComponentBeginOverlap(Explosion)
  (params (OverlappedComponent :type Primitive%20Component%20Object%20Reference) (OtherActor :type Actor%20Object%20Reference) (OtherComp :type Primitive%20Component%20Object%20Reference) (OtherBodyIndex :type Integer) (bFromSweep :type Boolean) (SweepResult :type Hit%20Result%20Structure%20%28by%20ref%29))
  (bind _asbasic_enemy (Utilities|Casting|CastToBasicEnemy OtherActor))
  (Collision|SetCollisionEnabled (Variables|Default|GetExplosion) "NoCollision")
  (Default|TakeDamage _asbasic_enemy (Variables|Default|GetDamage))
  (Actor|DestroyActor))

(event Custom|Explode
  (Effects|SpawnEmitteratLocation "/Game/InfinityBladeEffects/Effects/FX_Monsters/FX_Monster_Gruntling/FlameThrower/P_FlameExplode.P_FlameExplode" (Transformation|GetActorLocation))
  (Collision|SetCollisionEnabled (Variables|Default|GetExplosion) "QueryOnly")
  (Utilities|FlowControl|Delay 0.2)
  (Actor|DestroyActor))

(event EventBeginPlay)

(fn ConstructionScript
  (Collision|SetCollisionEnabled (Variables|Default|GetExplosion) "NoCollision"))